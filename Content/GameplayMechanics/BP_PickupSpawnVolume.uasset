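; BP_PickupSpawnVolume is a spawn volume that spawns one actor, with an ice upheaval particle effect, shortly after play begins.
; BeginPlay waits briefly, then passes GetSpawnActor and GetSpawnPoint results to SpawnOurActor.
; The SpawnOurActor override plays the emitter at that location, then calls the parent implementation to handle the spawn.
; A direct SpawnActor node using PawnToSpawn is left unconnected and never runs.
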(event EventBeginPlay
  (Utilities|FlowControl|Delay 0.2)
  (Class|SpawnVolume|SpawnOurActor (Class|SpawnVolume|GetSpawnActor) (Class|SpawnVolume|GetSpawnPoint)))

(event Collision|EventActorBeginOverlap
  (params (OtherActor :type Actor%20Object%20Reference)))

(event EventTick
  (params (DeltaSeconds :type Float%20%28single-precision%29)))

(event EventSpawnOurActor
  (params (ToSpawn :type Object%20Class%20Reference) (Location :type Vector%20%28by%20ref%29 :default "0, 0, 0"))
  (Effects|SpawnEmitteratLocation "/Game/InfinityBladeEffects/Effects/FX_Skill_Aura/P_Aura_Ice_Upheaval_01.P_Aura_Ice_Upheaval_01" Location)
  (|CallParentFunction ToSpawn Location))

(fn ConstructionScript)