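; Floor switch Blueprint that animates a pressure switch and its linked door with timelines.
; Lower switch and raise door events play their timelines, feeding each update to UpdateFloorSwitchLocation and UpdateDoorLocation, which are defined outside this graph.
; The opposite events reverse the same timelines to return switch and door.
; Nothing in this graph triggers these events, and a leftover door SetWorldLocation node is unconnected.
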(event EventBeginPlay)

(event Collision|EventActorBeginOverlap
  (params (OtherActor :type Actor%20Object%20Reference)))

(event EventTick
  (params (DeltaSeconds :type Float%20%28single-precision%29)))

(event EventRaiseDoor
  (bind _doorelevation (Timeline|DoorTimeline Play)
    (:Update
      (Class|FloorSwitch|UpdateDoorLocation _doorelevation))))

(event EventLowerDoor
  (bind _doorelevation (Timeline|DoorTimeline Reverse)
    (:Update
      (Class|FloorSwitch|UpdateDoorLocation _doorelevation))))

(event EventLowerFloorSwitch
  (bind _newtrack_0 (Timeline|FloorSwitchTimeline Play)
    (:Update
      (Class|FloorSwitch|UpdateFloorSwitchLocation _newtrack_0))))

(event EventRaiseFloorSwitch
  (bind _newtrack_0 (Timeline|FloorSwitchTimeline Reverse)
    (:Update
      (Class|FloorSwitch|UpdateFloorSwitchLocation _newtrack_0))))

(fn ConstructionScript)